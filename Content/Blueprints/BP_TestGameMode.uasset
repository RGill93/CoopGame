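; Test game mode that spawns AI bots and awards score for killing them.
; SpawnNewBot runs an EQS spawn-location query, using RandomBest25Pct, and works with its results to draw debug spheres and spawn a randomly weighted AdvancedAI or TrackerBot, favoring the tracker.
; An OnActorKilled handler, bound at BeginPlay, adds score to the killer's SPlayerState when the victim is a non-player pawn, then prints the total.
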(event Custom|OnQueryFinishedEvent_Event_0
  (params (QueryInstance :type Env%20Query%20Instance%20Blueprint%20Wrapper%20Object%20Reference) (QueryStatus :type EEnvQueryStatus%20Enum :default "Processing"))
  (switch Utilities|FlowControl|Switch|SwitchonEEnvQueryStatus QueryStatus))

(event Custom|OnActorKilled_Event_0
  (params (VictimActor :type Actor%20Object%20Reference) (KilledActor :type Actor%20Object%20Reference) (KillerController :type Controller%20Object%20Reference))
  (bind _aspawn (Utilities|Casting|CastToPawn VictimActor))
  (if (not (Pawn|IsPlayerControlled _aspawn))
    (bind _assplayer_state (Utilities|Casting|CastToSPlayerState (Variables|/Script/Engine.Pawn|GetPlayerState (Pawn|GetControlledPawn KillerController))))
    (Class|SPlayerState|AddScore _assplayer_state 2e+01)
    (Development|PrintString (Utilities|String|ToString(Float) (Variables|/Script/Engine.PlayerState|GetScore _assplayer_state)) true true "(R=0.776042,G=0.000000,B=0.041128,A=1.000000)")))

(event EventSpawnNewBot
  (bind _returnvalue (AI|EQS|RunEQSQuery "/Game/Blueprints/EQS_FindSpawnLocation.EQS_FindSpawnLocation" self "RandomBest25Pct"))
  (EventDispatchers|AssignOnQueryFinishedEvent _returnvalue (delegate Custom|OnQueryFinishedEvent_Event_0))
  (for _array_element (Class|EnvQueryInstanceBlueprintWrapper|GetResultsasLocations (stale Custom|OnQueryFinishedEvent_Event_0 QueryInstance))
    (Rendering|Debug|DrawDebugSphere _array_element 5e+01 12 "(R=1.000000,G=0.949198,B=0.000000,A=1.000000)" 2.0 2.0)
    (Game|SpawnActorfromClass (select (<= (Math|Random|RandomFloatinRange 0.0 1e+02) 35.0) "/Game/AdvancedAI/BP_AdvancedAI.BP_AdvancedAI_C" "/Game/TrackerBot/BP_TrackerBot.BP_TrackerBot_C") (Math|Transform|MakeTransform _array_element) "AdjustIfPossibleButDontSpawnIfColliding" 0 0)))

(event EventBeginPlay
  (EventDispatchers|AssignOnActorKilled (delegate Custom|OnActorKilled_Event_0)))

(fn ConstructionScript)